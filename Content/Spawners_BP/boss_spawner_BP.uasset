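; Boss spawner that runs an endless ghost-spawning loop from BeginPlay, after passing its spawn interval to the FirstPersonCharacter.
; Each cycle places a Box_of_pain_BP at a random target, waits the interval, then spawns one of two ghost types there.
; When the spawn counter reaches Bar, it resets and spawns a Special_ghost instead, plays an appearance sound at a re-rolled target and pauses longer before looping.
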(event EventBeginPlay
  (bind _set_of_targets (Variables|Default|Getset_of_targets))
  (bind _returnvalue (Utilities|Array|Length _set_of_targets))
  (bind _returnvalue_2 (Math|Random|RandomInteger _returnvalue))
  (bind _output (Utilities|Array|Get(acopy) _set_of_targets _returnvalue_2))
  (bind _returnvalue_3 (Transformation|GetActorLocation _output))
  (bind _asfirst_person_character (Utilities|Casting|CastToFirstPersonCharacter (Game|GetPlayerCharacter 0)))
  (Variables|/Game/FirstPersonBP/Blueprints/FirstPersonCharacter.FirstPersonCharacter_C|Settime_for_spawner _asfirst_person_character (Variables|Default|Gettime_between_spawns))
  (Variables|Default|Settransformerss (Math|Transform|MakeTransform _returnvalue_3) :!label _label)
  (Game|SpawnActorfromClass "/Game/Spawners_BP/box_of_pain_BP.box_of_pain_BP_C" (Variables|Default|Gettransformerss) "Undefined" 0 0)
  (if (== (Variables|Default|Getspawn_before_shiny) (Variables|Default|Getbar))
    ;[1 1 1] spawnowanie specialnego duszka
    (Variables|Default|Setspawn_before_shiny 0)
    (Utilities|FlowControl|Delay (Variables|Default|Gettime_between_spawns))
    (Game|SpawnActorfromClass "/Game/enemies_BP/special_ghost.special_ghost_C" (Variables|Default|Gettransformerss) "Undefined" 0 0)
    (Audio|PlaySoundatLocation "/Game/Textures_and_meshes/sfx/appearingghost.appearingghost" _returnvalue_3 "0, 0, 0" 1.0 1.0 0.0 0 0 0)
    (Utilities|FlowControl|Delay 15.0)
    (goto _label)
    (else
      (Utilities|FlowControl|Delay (Variables|Default|Gettime_between_spawns))
      (if (Math|Random|RandomBool)
        (Game|SpawnActorfromClass "/Game/enemies_BP/Ghost_BP.Ghost_BP_C" (Variables|Default|Gettransformerss) "Undefined" 0 0)
        (else
          (Game|SpawnActorfromClass "/Game/enemies_BP/Ghost_BP2.Ghost_BP2_C" (Variables|Default|Gettransformerss) "Undefined" 0 0)))
      (Variables|Default|Setspawn_before_shiny (+ (Variables|Default|Getspawn_before_shiny) 1))
      (goto _label))))

(event Collision|EventActorBeginOverlap
  (params (OtherActor :type Actor%20Object%20Reference)))

(fn ConstructionScript)