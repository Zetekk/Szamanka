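; Portal Blueprint that moves the player to the intermediate map once enough special-ghost lamps are collected.
; When the first-person character overlaps its Box with at least three lamps, it resets that count, calls RemoveMelodies on the player and opens "mapa_posrednia".
; Otherwise it shows a Souls1BP widget on screen for a second, then removes it.
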(event OnComponentBeginOverlap(Box)
  (params (OverlappedComponent :type Primitive%20Component%20Object%20Reference) (OtherActor :type Actor%20Object%20Reference) (OtherComp :type Primitive%20Component%20Object%20Reference) (OtherBodyIndex :type Integer) (bFromSweep :type Boolean) (SweepResult :type Hit%20Result%20Structure%20%28by%20ref%29))
  (bind _asfirst_person_character (Utilities|Casting|CastToFirstPersonCharacter OtherActor))
  (if (>= (Variables|/Game/FirstPersonBP/Blueprints/FirstPersonCharacter.FirstPersonCharacter_C|Getlampies_from_special_ghosts _asfirst_person_character) 3)
    (Variables|/Game/FirstPersonBP/Blueprints/FirstPersonCharacter.FirstPersonCharacter_C|Setlampies_from_special_ghosts _asfirst_person_character 0)
    (bind _asfirst_person_character_2 (Utilities|Casting|CastToFirstPersonCharacter (Game|GetPlayerCharacter 0)))
    (Default|RemoveMelodies _asfirst_person_character_2)
    (Game|OpenLevel(byName) "mapa_posrednia")
    (else
      (bind _returnvalue (UserInterface|CreateWidget "/Game/UI/Souls1BP.Souls1BP_C"))
      (UserInterface|Viewport|AddtoViewport _returnvalue 0)
      (Utilities|FlowControl|Delay 1.0)
      (Widget|RemovefromParent _returnvalue))))

(event EventBeginPlay)

(event Collision|EventActorBeginOverlap
  (params (OtherActor :type Actor%20Object%20Reference)))

(event EventTick
  (params (DeltaSeconds :type Float%20%28single-precision%29)))

(fn ConstructionScript)