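; Box of pain is a timed actor that destroys itself shortly after play begins, using the first-person player character's TimeForSpawner value, less a small margin, as its lifetime.
; Its disconnected nodes hold an unused spawner that would pick a random target location, spawn one of two ghost variants there when a flag is set, then destroy itself.
; As wired, only the delayed self-destruction runs.
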(event EventBeginPlay
  (bind _asfirst_person_character (Utilities|Casting|CastToFirstPersonCharacter (Game|GetPlayerCharacter 0)))
  (Utilities|FlowControl|Delay (- (Variables|/Game/FirstPersonBP/Blueprints/FirstPersonCharacter.FirstPersonCharacter_C|Gettime_for_spawner _asfirst_person_character) 0.01))
  (Actor|DestroyActor))

(fn ConstructionScript)