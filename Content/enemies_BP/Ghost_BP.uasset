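; Ghost enemy that chases the first-person player and damages them on contact.
; From BeginPlay it reissues an AI move toward the player character every 0.2 seconds through a looping delay.
; An overlap on its sphere component removes one HP from the player, then destroys the ghost if the player survives.
; At zero HP it instead shows the cursor, switches to UI-only input and opens the game-over level.
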(event OnComponentBeginOverlap(Sphere1)
  (params (OverlappedComponent :type Primitive%20Component%20Object%20Reference) (OtherActor :type Actor%20Object%20Reference) (OtherComp :type Primitive%20Component%20Object%20Reference) (OtherBodyIndex :type Integer) (bFromSweep :type Boolean) (SweepResult :type Hit%20Result%20Structure%20%28by%20ref%29))
  (bind _returnvalue (Game|GetPlayerController 0))
  ;[1 1 1] damaging player on contac
  (bind _asfirst_person_character (Utilities|Casting|CastToFirstPersonCharacter OtherActor))
  (Variables|/Game/FirstPersonBP/Blueprints/FirstPersonCharacter.FirstPersonCharacter_C|SetHP_left _asfirst_person_character (- (Variables|/Game/FirstPersonBP/Blueprints/FirstPersonCharacter.FirstPersonCharacter_C|GetHP_left _asfirst_person_character) 1))
  (if (<= (Variables|/Game/FirstPersonBP/Blueprints/FirstPersonCharacter.FirstPersonCharacter_C|GetHP_left _asfirst_person_character) 0)
    ;[1 1 1] reseting game
    (Variables|/Script/Engine.PlayerController|SetbShowMouseCursor _returnvalue true)
    (Input|SetInputModeUIOnly _returnvalue 0 "DoNotLock")
    (Game|OpenLevel(byName) "Game_over_world")
    (else
      (Actor|DestroyActor))))

(event EventBeginPlay
  (bind _asfirst_person_character (Utilities|Casting|CastToFirstPersonCharacter (Game|GetPlayerCharacter 0)))
  (AI|AIMoveTo self "0, 0, 0" _asfirst_person_character 5.0 false :!label _label
    (:then
      (Utilities|FlowControl|Delay 0.2)
      (goto _label))))

(event Collision|EventActorBeginOverlap
  (params (OtherActor :type Actor%20Object%20Reference)))

(event EventTick
  (params (DeltaSeconds :type Float%20%28single-precision%29)))

(fn ConstructionScript)